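; AI controller for guard NPCs that aim and shoot at perceived targets.
; On BeginPlay it sets up the PatrolData blackboard and runs the Guard_Behavior tree.
; Perception updates for any actor without the "Enemy" tag set FocusPawn and switch on the controlled Ue4ASP_Character's Aiming and Shooting flags when sensed.
; When sensing fails for such an actor, it clears FocusPawn and both flags.
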(event `self.ReceiveBeginPlay`
  (bind _blackboardcomponent (`self.UseBlackboard` "/Game/Dynamic/NPC/AI/PatrolData.PatrolData"))
  (set `self.BlackboardComponent` _blackboardcomponent)
  (`self.RunBehaviorTree` "/Game/Dynamic/NPC/AI/Guard_Behavior.Guard_Behavior"))

(event `self.AIPerception.OnTargetPerceptionUpdated`
  (params (Actor :type "Actor Object Reference") (Stimulus :type "AIStimulus Structure"))
  (bind _returnvalue (`self.K2_GetPawn`))
  (bind _blackboardcomponent (`self.BlackboardComponent`))
  (bind _focuspawn (`self.FocusPawn`))
  (if (`self.ActorHasTag` Actor "Enemy")
    _
    (elif (`.bSuccessfullySensed` (break `AIStimulus` Stimulus))
      (`BlackboardComponent.SetValueAsObject` _blackboardcomponent _focuspawn Actor)
      (bind _asue_4asp_character (cast `/Game/Dynamic/NPC/Behavior/Ue4ASP_Character` _returnvalue))
      (set `/Game/Dynamic/NPC/Behavior/Ue4ASP_Character.Aiming` true _asue_4asp_character)
      (set `/Game/Dynamic/NPC/Behavior/Ue4ASP_Character.Shooting` true _asue_4asp_character)
      (else
        (`BlackboardComponent.ClearValue` _blackboardcomponent _focuspawn)
        (bind _asue_4asp_character_2 (cast `/Game/Dynamic/NPC/Behavior/Ue4ASP_Character` _returnvalue))
        (set `/Game/Dynamic/NPC/Behavior/Ue4ASP_Character.Aiming` false _asue_4asp_character_2)
        (set `/Game/Dynamic/NPC/Behavior/Ue4ASP_Character.Shooting` false _asue_4asp_character_2)))))

(fn `UserConstructionScript`)